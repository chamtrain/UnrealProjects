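; BHSCharacter is a bot character Blueprint that takes damage and explodes when its health runs out.
; AnyDamage subtracts Health, then either rescales the HealthBar along Y by health ratio or triggers Explode.
; Explode spawns an emitter at the actor, plays a sound at world origin and destroys the actor.
; The construction script assigns high and low health materials, but the material-swap branch is disconnected, so only scaling runs.
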(event `DeadEvent`
  (`self.Explode`))

(event `RescaleHealthBarEvent`
  (`self.Rescale Health Bar`))

(event `self.ReceiveAnyDamage`
  (params (Damage :type "Float (single-precision)") (DamageType :type "DamageType Object Reference") (InstigatedBy :type "Controller Object Reference") (DamageCauser :type "Actor Object Reference"))
  (bind _returnvalue (- (`self.Health`) Damage))
  (if (> _returnvalue 0.0)
    (set `self.Health` _returnvalue)
    (`self.RescaleHealthBarEvent`)
    (else
      (set `self.Health` 0.0)
      (`self.DeadEvent`))))

(fn `Explode`
  (`GameplayStatics.SpawnEmitterAtLocation` null "/Game/StarterContent/Particles/P_Explosion.P_Explosion" (`self.K2_GetActorLocation`))
  (`GameplayStatics.PlaySoundAtLocation` null "/Game/StarterContent/Audio/Explosion02.Explosion02")
  (`self.K2_DestroyActor`))

(fn `Rescale Health Bar`
  (`SceneComponent.SetWorldScale3D` (`self.HealthBar`) (`KismetMathLibrary.MakeVector` 0.07 (/ (`self.Health`) (`self.HealthMax`)) 0.07)))

(fn `UserConstructionScript`
  (set `self.HighHealth` "/Game/SpeedTree/Christmas_Tree_Desktop_Meshes_Mat.Christmas_Tree_Desktop_Meshes_Mat")
  (set `self.LowHealth` "/Game/SpeedTree/Christmas_Tree_Desktop_Meshes_2_Mat.Christmas_Tree_Desktop_Meshes_2_Mat"))