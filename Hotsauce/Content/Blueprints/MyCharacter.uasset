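; MyCharacter is a Blueprint that acts as a damage aura, hurting nearby BHSCharacter actors.
; Every Tick it gathers all BHSCharacter actors, skips itself and applies a fixed damage to each one within a set radius.
; The damage is applied per frame without delta-time scaling, so its rate depends on frame rate.
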(event `self.ReceiveTick`
  (params (DeltaSeconds :type "Float (single-precision)"))
  (bind _outactors (`GameplayStatics.GetAllActorsOfClass` null "/Game/Blueprints/Bots/BHSCharacter.BHSCharacter_C"))
  (for _array_element _outactors
    (if (== self _array_element)
      _
      (elif (< (`KismetMathLibrary.VSize` (- (`self.K2_GetActorLocation` _array_element) (`self.K2_GetActorLocation`))) 500.0)
        (`GameplayStatics.ApplyDamage` _array_element 5.0)))))

(fn `UserConstructionScript`)